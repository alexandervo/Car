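; Player-driven truck Blueprint that moves and yaws through Enhanced Input (IMC_Car) and shows a minimap widget from BeginPlay.
; M opens a location-select widget with the mouse cursor, using an IsOpen flag that only resets on a later press once the cursor is hidden.
; T asks BPWaypoint to create a periodically updated waypoint toward a randomly chosen AI_Draw actor.
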(event Input|EnhancedActionEvents|EnhancedInputActionMove
  (params (ActionValue :type Vector%202D%20Structure) (ElapsedSeconds :type Float%20%28double-precision%29) (TriggeredSeconds :type Float%20%28double-precision%29) (InputAction :type Input%20Action%20Object%20Reference :default "/Game/Blueprints/Move.Move"))
  (bind _returnvalue (Pawn|GetControlRotation :!class /Script/Engine.Pawn))
  ;[1 1 1] Move Around
  (Pawn|Input|AddMovementInput (Math|Vector|GetRightVector (Pawn|GetControlRotation :!class /Script/Engine.Pawn)) (.x ActionValue) false)
  (Pawn|Input|AddMovementInput (Math|Vector|GetForwardVector (Math|Rotator|MakeRotator (.roll _returnvalue) 0.0 (.yaw _returnvalue))) (.y ActionValue) false))

(event Input|EnhancedActionEvents|EnhancedInputActionLook_around
  (params (ActionValue :type Vector%202D%20Structure) (ElapsedSeconds :type Float%20%28double-precision%29) (TriggeredSeconds :type Float%20%28double-precision%29) (InputAction :type Input%20Action%20Object%20Reference :default "/Game/Blueprints/Look_around.Look_around"))
  (Pawn|Input|AddControllerYawInput (.x ActionValue)))

(event EventBeginPlay
  ;[1 1 1] Active
  (bind _asplayer_controller (Utilities|Casting|CastToPlayerController (Game|GetPlayerController 0)))
  (Utilities|IsValid (PlayerController|LocalPlayerSubsystems|GetEnhancedInputLocalPlayerSubsystem _asplayer_controller)
    (:Is%20Valid
      (Input|AddMappingContext (PlayerController|LocalPlayerSubsystems|GetEnhancedInputLocalPlayerSubsystem _asplayer_controller) "/Game/Blueprints/IMC_Car.IMC_Car" 0 "(bIgnoreAllPressedKeysUntilRelease=True,bForceImmediately=False,bNotifyUserSettings=False)")
      (bind _returnvalue (UserInterface|CreateWidget "/Game/Blueprints/W_Minimap.W_Minimap_C"))
      (UserInterface|Viewport|AddtoViewport _returnvalue 0)
      (Variables|Default|SetIsOpen false))))

(event Input|KeyboardEvents|M
  (params (Key :type Key%20Structure :default "None"))
  (bind _returnvalue (Game|GetPlayerController 0))
  (:Pressed
    (bind _returnvalue_2 (UserInterface|CreateWidget "/Game/Blueprints/W_LocationSelect.W_LocationSelect_C"))
    (if (Variables|Default|GetIsOpen)
      (if (not (Variables|/Script/Engine.PlayerController|GetbShowMouseCursor _returnvalue))
        (Variables|Default|SetIsOpen false))
      (else
        (Variables|Default|SetIsOpen true)
        (UserInterface|Viewport|AddtoViewport _returnvalue_2 0)
        (Variables|/Script/Engine.PlayerController|SetbShowMouseCursor _returnvalue true)))))

(event Input|KeyboardEvents|T
  (params (Key :type Key%20Structure :default "None"))
  (:Pressed
    (bind _outactors (Actor|GetAllActorsOfClass "/Game/Blueprints/AI_Draw.AI_Draw_C"))
    (Default|CreateWayPoint (Variables|Default|GetBP_Waypoint) (Transformation|GetActorLocation (.OutItem (Utilities|Array|Random _outactors))) 1.5e+02 0.4 2.5e+02 3e+01)))

(fn ConstructionScript)